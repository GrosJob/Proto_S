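; FlashLight_BP is a toggleable, battery-powered flashlight using a RectLight.
; Each tick it drains energy while lit, switching off at empty, and recharges during daytime as signaled by the ProtoS_GameState day/night event.
; When energy falls to a low fraction of maximum, DoOnce gates trigger a timeline that modulates light intensity as a low-battery effect.
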(event Custom|FlashLightInUse
  ;[0.3536 1 0.4188] Regene / Use / Low battery effect
  (if (and (Variables|Default|GetlightOn) (> (Variables|Default|GetflashLightEnergy) 0.0))
    (bind _output_get (Variables|Default|SetflashLightEnergy (select (< (- (Variables|Default|GetflashLightEnergy) (* (Utilities|Time|GetWorldDeltaSeconds) 5.0)) 0.0) 0.0 (- (Variables|Default|GetflashLightEnergy) (* (Utilities|Time|GetWorldDeltaSeconds) 5.0)))))
    (Variables|Default|SetlowBatterry (<= _output_get (* (Variables|Default|GetflashLightMaxEnergy) 0.2)))
    (if (== _output_get 0.0)
      (Variables|Default|SetlightOn false)
      (Rendering|SetVisibility (Variables|Default|GetRectLight) false false))))

(event Custom|ChargeLight
  (bind _flashlightmaxenergy (Variables|Default|GetflashLightMaxEnergy))
  ;[0.3536 1 0.4188] Regene / Use / Low battery effect
  (if (and (Variables|Default|GetflashLightReload) (< (Variables|Default|GetflashLightEnergy) (Variables|Default|GetflashLightMaxEnergy)))
    (Variables|Default|SetflashLightEnergy (select (> (+ (Variables|Default|GetflashLightEnergy) (* (Utilities|Time|GetWorldDeltaSeconds) 3.0)) _flashlightmaxenergy) _flashlightmaxenergy (+ (Variables|Default|GetflashLightEnergy) (* (Utilities|Time|GetWorldDeltaSeconds) 3.0))))))

(event Custom|SwichLight
  ;[0.5355 0.5535 1] Switch Light
  (if (> (Variables|Default|GetflashLightEnergy) 0.0)
    (bind _output_get (Variables|Default|SetlightOn (not (Variables|Default|GetlightOn))))
    (Utilities|FlowControl|Sequence
      (:then_0
        (if (not _output_get)
          ;[0.3536 1 0.4188] Regene / Use / Low battery effect
          (bind _intensity (Timeline|Timeline_0 Stop)
            (:Update
              (Rendering|Components|Light|SetIntensity (Variables|Default|GetRectLight) (Math|Float|Lerp 0.0 (Variables|Default|GetintensityMax) _intensity))))))
      (:then_1
        (Rendering|SetVisibility (Variables|Default|GetRectLight) _output_get false)
        (Rendering|Components|Light|SetIntensity (Variables|Default|GetRectLight) (Variables|Default|GetintensityMax))))))

(event Custom|VerifyBattery
  ;[0.3536 1 0.4188] Regene / Use / Low battery effect
  (if (Variables|Default|GetlowBatterry)
    (Utilities|FlowControl|DoOnce false :!label _label
      (:Completed
        (Utilities|FlowControl|Sequence
          (:then_0
            (bind _intensity (Timeline|Timeline_0 PlayFromStart)
              (:Update
                (Rendering|Components|Light|SetIntensity (Variables|Default|GetRectLight) (Math|Float|Lerp 0.0 (Variables|Default|GetintensityMax) _intensity)))))
          (:then_1
            (goto _label_2 Reset)))))
    (else
      (Utilities|FlowControl|DoOnce false :!label _label_2
        (:Completed
          (Utilities|FlowControl|Sequence
            (:then_0
              (goto _label Reset))
            (:then_1
              (Timeline|Timeline_0 Stop))))))))

(event Custom|DayNightEvent
  ;[1 0.292 0.3606] Begin Play / Event Tick
  (Variables|Default|SetflashLightReload (not (Variables|/Game/Survive/Core/ProtoS_GameState.ProtoS_GameState_C|GetisNightTime (Variables|Default|GetgameState_ref)))))

(event EventBeginPlay
  (bind _returnvalue (Game|GetGameState))
  (bind _asproto_s_game_state (Utilities|Casting|CastToProtoS_GameState _returnvalue))
  ;[1 0.292 0.3606] Begin Play / Event Tick
  (Variables|Default|SetintensityMax (Variables|/Script/Engine.LightComponentBase|GetIntensity (Variables|Default|GetRectLight)))
  (Variables|Default|SetflashLightEnergy (Variables|Default|GetflashLightMaxEnergy))
  (bind _output_get (Variables|Default|SetgameState_ref _asproto_s_game_state))
  (EventDispatchers|BindEventtoNewDayNight _asproto_s_game_state (delegate Custom|DayNightEvent)))

(event EventTick
  (params (DeltaSeconds :type Float%20%28single-precision%29))
  ;[1 0.292 0.3606] Begin Play / Event Tick
  (Utilities|FlowControl|Sequence
    (:then_0
      (CallFunction|FlashLightinUse))
    (:then_1
      (CallFunction|ChargeLight))
    (:then_2
      (CallFunction|VerifyBattery))))

(fn ConstructionScript)